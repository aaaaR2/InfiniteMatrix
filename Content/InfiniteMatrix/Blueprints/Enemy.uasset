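; Enemy actor that spins in place and reacts when its EnemyModel component is overlapped.
; Tick rotates the model on all three axes, scaled by RotateSpeed and delta time.
; Touching BP_Player decreases its health, destroys the enemy and shows restart if the player is dead.
; A BP_Projectile hit increments the GM_Tutorial score, then destroys both projectile and enemy.
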(event `self.ReceiveBeginPlay`)

(event `self.ReceiveTick`
  (params (DeltaSeconds :type "Float (single-precision)"))
  (bind _returnvalue (* DeltaSeconds (`self.RotateSpeed`)))
  (`SceneComponent.K2_AddLocalRotation` (`self.EnemyModel`) (`KismetMathLibrary.MakeRotator` _returnvalue _returnvalue _returnvalue) false false))

(event `self.EnemyModel.OnComponentBeginOverlap`
  (params (OverlappedComponent :type "PrimitiveComponent Object Reference") (OtherActor :type "Actor Object Reference") (OtherComp :type "PrimitiveComponent Object Reference") (OtherBodyIndex :type Integer) (bFromSweep :type Boolean) (SweepResult :type "HitResult Structure (by ref)"))
  (bind _asbp_player (cast `/Game/InfiniteMatrix/Blueprints/BP_Player` OtherActor)
    (:`then`
      (`/Game/InfiniteMatrix/Blueprints/BP_Player.DecreaseHealth` _asbp_player)
      (`self.K2_DestroyActor`)
      (if (`/Game/InfiniteMatrix/Blueprints/BP_Player.IsDead` _asbp_player)
        (`/Game/InfiniteMatrix/Blueprints/BP_Player.DisplayRestart` _asbp_player)))
    (:`CastFailed`
      (bind _asbp_projectile (cast `/Game/InfiniteMatrix/Blueprints/BP_Projectile` OtherActor))
      (bind _asgm_tutorial (cast `/Game/InfiniteMatrix/Blueprints/GM_Tutorial` (`GameplayStatics.GetGameMode`)))
      (`/Game/InfiniteMatrix/Blueprints/GM_Tutorial.IncrementPlayerScore` _asgm_tutorial)
      (`self.K2_DestroyActor` _asbp_projectile)
      (`self.K2_DestroyActor`))))

(fn `UserConstructionScript`)