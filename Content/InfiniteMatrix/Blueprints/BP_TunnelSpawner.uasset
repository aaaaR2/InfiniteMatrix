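; BP_TunnelSpawner builds a chain of BP_Tunnel segments and populates them with enemies and health packs.
; On BeginPlay it clears existing tunnels and enemies, then spawns a stretched segment at the player, with further segments at the newest one's SpawnPoint.
; Each segment gets a spawner back-reference, a randomized wall and chance-based pickup and enemy spawns at random offsets.
; Spawned enemies and packs expire after a short lifespan.
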(event `self.ReceiveBeginPlay`
  (`self.SpawnInitialTunnels`))

(fn `SpawnEnemies`
  (params (DefaultSpawnLocation :type "Vector Structure"))
  (bind _returnvalue (`KismetMathLibrary.RandomFloatInRange` -400.0 400.0))
  (bind _returnvalue_2 (- 400.0 (`KismetMathLibrary.Abs` _returnvalue)))
  (for _ (range (+ (`KismetMathLibrary.RandomIntegerInRange` 0 1) 1))
    (bind _returnvalue_3 (`|SpawnActorFromClass` "/Game/InfiniteMatrix/Blueprints/Enemy.Enemy_C" (`KismetMathLibrary.MakeTransform` (`KismetMathLibrary.TransformLocation` (`KismetMathLibrary.MakeTransform` (`KismetMathLibrary.MakeVector` (`KismetMathLibrary.RandomFloatInRange` 500.0 2400.0) _returnvalue (`KismetMathLibrary.RandomFloatInRange` (* -1 _returnvalue_2) (* 1 _returnvalue_2)))) DefaultSpawnLocation)) "Undefined" "OverrideRootScale" null null))
    (`self.SetLifeSpan` _returnvalue_3 5.0)))

(fn `SpawnHealthPack`
  (params (`Spawn Location` :type "Vector Structure"))
  (bind _returnvalue (`KismetMathLibrary.RandomFloatInRange` -400.0 400.0))
  (bind _returnvalue_2 (- 400.0 (`KismetMathLibrary.Abs` _returnvalue)))
  (if (== (`KismetMathLibrary.RandomIntegerInRange` 0 9) 0)
    (bind _returnvalue_3 (`|SpawnActorFromClass` "/Game/InfiniteMatrix/Blueprints/HealthPack.HealthPack_C" (`KismetMathLibrary.MakeTransform` (`KismetMathLibrary.TransformLocation` (`KismetMathLibrary.MakeTransform` (`KismetMathLibrary.MakeVector` (`KismetMathLibrary.RandomFloatInRange` 1000.0 2400.0) _returnvalue (`KismetMathLibrary.RandomFloatInRange` (* -1 _returnvalue_2) (* 1 _returnvalue_2)))) `Spawn Location`)) "Undefined" "OverrideRootScale" null null))
    (`self.SetLifeSpan` _returnvalue_3 5.0)))

(fn `SpawnInitialTunnels`
  (`|ExecutionSequence`
    (:`then_0`
      (bind _outactors (`GameplayStatics.GetAllActorsOfClass` "/Game/InfiniteMatrix/Blueprints/BP_Tunnel.BP_Tunnel_C"))
      (for _array_element _outactors
        (`self.K2_DestroyActor` _array_element)
        (bind _outactors_2 (`GameplayStatics.GetAllActorsOfClass` "/Game/InfiniteMatrix/Blueprints/Enemy.Enemy_C"))
        (for _array_element_2 _outactors_2
          (`self.K2_DestroyActor` _array_element_2))))
    (:`then_1`
      (for _ (range 3)
        (`/Engine/EditorBlueprintResources/StandardMacros.IsValid` (`self.NewestTunnel`)
          (:`Is Valid`
            (`self.SpawnTunnelAtSpawnPoint`))
          (:`Is Not Valid`
            (`self.SpawnTunnel` (`self.K2_GetActorLocation` (`GameplayStatics.GetPlayerPawn` 0)) (2.0 1.0 1.0))))))))

(fn `SpawnTunnel`
  (params (SpawnLocation :type "Vector Structure") (TransformScale :type "Vector Structure"))
  (bind _returnvalue (`|SpawnActorFromClass` "/Game/InfiniteMatrix/Blueprints/BP_Tunnel.BP_Tunnel_C" (`KismetMathLibrary.MakeTransform` SpawnLocation (struct) TransformScale) "Undefined" "OverrideRootScale" null null))
  (bind _output_get (set `self.NewestTunnel` _returnvalue))
  (set `/Game/InfiniteMatrix/Blueprints/BP_Tunnel.TunnelSpawner` self _output_get)
  (`self.SpawnHealthPack` self (`SceneComponent.K2_GetComponentLocation` (`/Game/InfiniteMatrix/Blueprints/BP_Tunnel.HealthPackSpawnPoint` _output_get)))
  (`self.SpawnEnemies` (`SceneComponent.K2_GetComponentLocation` (`/Game/InfiniteMatrix/Blueprints/BP_Tunnel.DefaultEnemySpawnPoint` _output_get)))
  (`/Game/InfiniteMatrix/Blueprints/BP_Tunnel.RandomizeWall` _output_get))

(fn `SpawnTunnelAtSpawnPoint`
  (`self.SpawnTunnel` (`SceneComponent.K2_GetComponentLocation` (`/Game/InfiniteMatrix/Blueprints/BP_Tunnel.SpawnPoint` (`self.NewestTunnel`))) (1.0 1.0 1.0)))

(fn `UserConstructionScript`)