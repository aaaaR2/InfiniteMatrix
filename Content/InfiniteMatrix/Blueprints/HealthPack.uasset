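; HealthPack is a pickup Blueprint that restores one point of health to the player.
; When a BP_Player overlaps its Sphere, it adds one to CurrentHealth if that is below MaxHealth.
; The pack destroys itself on any player overlap, so it is consumed even at full health.
; Its Destroyed event spawns an emitter at the actor's location.
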(event `self.Sphere.OnComponentBeginOverlap`
  (params (OverlappedComponent :type "PrimitiveComponent Object Reference") (OtherActor :type "Actor Object Reference") (OtherComp :type "PrimitiveComponent Object Reference") (OtherBodyIndex :type Integer) (bFromSweep :type Boolean) (SweepResult :type "HitResult Structure (by ref)"))
  (bind _asbp_player (cast `/Game/InfiniteMatrix/Blueprints/BP_Player` OtherActor))
  (bind _currenthealth (`/Game/InfiniteMatrix/Blueprints/BP_Player.CurrentHealth` _asbp_player))
  (if (< _currenthealth (`/Game/InfiniteMatrix/Blueprints/BP_Player.MaxHealth` _asbp_player))
    (set `/Game/InfiniteMatrix/Blueprints/BP_Player.CurrentHealth` (+ _currenthealth 1) _asbp_player)
    (`self.K2_DestroyActor`)
    (else
      (`self.K2_DestroyActor`))))

(event `self.ReceiveDestroyed`
  (`GameplayStatics.SpawnEmitterAtLocation` null (`self.K2_GetActorLocation`)))

(fn `UserConstructionScript`)